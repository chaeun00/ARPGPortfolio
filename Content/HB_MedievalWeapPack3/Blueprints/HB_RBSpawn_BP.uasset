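; Physics prop from a medieval weapon pack that displays a configurable static mesh and reacts to impacts with sparks.
; On Hit with SelfMoved and a passed VelocityValidation, it spawns sparks, waits briefly, re-arms, then drives angular damping through a timeline.
; The hit flag clears before validation, so a failed check leaves effects disabled.
; VelocityValidation holds a per-axis speed-limit comparison, marked unused.
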(event Collision|EventHit
  (params (MyComp :type Primitive%20Component%20Object%20Reference) (Other :type Actor%20Object%20Reference) (OtherComp :type Primitive%20Component%20Object%20Reference) (bSelfMoved :type Boolean) (HitLocation :type Vector :default "0, 0, 0") (HitNormal :type Vector :default "0, 0, 0") (NormalImpulse :type Vector :default "0, 0, 0") (Hit :type Hit%20Result%20Structure%20%28by%20ref%29))
  ;[1 1 1] Spawn Hit Sparks
  (if (Variables|Default|GetCanPlayHitEffect)
    (Variables|Default|SetCanPlayHitEffect false)
    (if (and (|VelocityValidation) bSelfMoved)
      (Effects|SpawnEmitteratLocation "/Game/HB_MedievalWeapPack3/Particles/HB_Sparks_01_PRT.HB_Sparks_01_PRT" HitLocation)
      (Utilities|FlowControl|RetriggerableDelay 0.5)
      (Variables|Default|SetCanPlayHitEffect true)
      (bind _angulardampen (Timeline|Timeline_0 PlayFromStart)
        (:Update
          (Class|PrimitiveComponent|SetAngularDamping (Variables|Default|GetStaticMesh1) _angulardampen))))))

(fn ConstructionScript
  (Components|StaticMesh|SetStaticMesh (Variables|Default|GetStaticMesh1) (Variables|Default|GetNewMesh)))